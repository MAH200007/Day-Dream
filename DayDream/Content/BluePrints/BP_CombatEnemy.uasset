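; BP_CombatEnemy is an enemy for turn-based combat that starts with a set Health value at BeginPlay.
; On its turn event it takes one point from the Player's Health, and its TakeDamage event subtracts a fixed amount from its own.
; The Death event checks for depleted Health but performs no action, and the not-my-turn event is empty.
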(event Custom|TakeDamage
  (Variables|Default|SetHealth (- (Variables|Default|GetHealth) 25)))

(event Custom|EIsMyTurn
  (bind _player (Variables|Default|GetPlayer))
  (Variables|/Game/BluePrints/BP_CombatPlayer.BP_CombatPlayer_C|SetHealth _player (- (Variables|/Game/BluePrints/BP_CombatPlayer.BP_CombatPlayer_C|GetHealth _player) 1)))

(event Custom|EIsNotMyTurn)

(event Custom|Death
  (if (<= (Variables|Default|GetHealth) 0)
    _))

(event EventBeginPlay
  (Variables|Default|SetHealth 100))

(event Collision|EventActorBeginOverlap
  (params (OtherActor :type Actor%20Object%20Reference)))

(event EventTick
  (params (DeltaSeconds :type Float%20%28single-precision%29)))

(fn ConstructionScript)